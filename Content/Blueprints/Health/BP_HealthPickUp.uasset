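; BP_HealthPickUp is a pickup actor that heals the arena character on touch.
; On overlap, it casts the other actor to BP_ArenaCharacter and restores a fixed amount of health.
; It then attaches an auto-destroying Niagara healing effect to the character mesh's spine and destroys itself.
; A failed cast only prints a debug message, leaving the pickup in place.
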(event EventBeginPlay
  (|CallParentFunction) ; This node is disabled and will not be called.\nDrag off pins to build functionality.
)

(event Collision|EventActorBeginOverlap
  (params (OtherActor :type Actor%20Object%20Reference))
  (bind _asbp_arena_character (Utilities|Casting|CastToBP_ArenaCharacter OtherActor)
    (:then
      (Default|RestoreHealth _asbp_arena_character 25.0)
      (Niagara|SpawnSystemAttached "/Game/sA_PickupSet_1/Fx/NiagaraSystems/NS_Healing_1.NS_Healing_1" (Variables|/Script/Engine.Character|GetMesh _asbp_arena_character) "Spine2" "0, 0, 0" "0, 0, 0" "KeepRelativeOffset" true)
      (Actor|DestroyActor))
    (:CastFailed
      (Development|PrintString "I am actually not casting bruv"))))

(event EventTick
  (params (DeltaSeconds :type Float%20%28single-precision%29))
  (|CallParentFunction DeltaSeconds) ; This node is disabled and will not be called.\nDrag off pins to build functionality.
)

(fn ConstructionScript
  (|CallParentFunction))